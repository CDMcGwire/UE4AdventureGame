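; Base character for movement, stick aiming, charge-limited dodges, melee combat and health.
; Dodges launch the character with altered friction and recharge on timers.
; Primary attack drives the anim blueprint; long press sphere-traces for a target and closes the gap by timeline, striking midway, while the airborne dive attack is an empty stub.
; Fist overlaps deal point damage; damage reddens a dynamic material, and death triggers ragdoll.
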(event `self.ReceiveBeginPlay`
  (bind _mesh (`self.Mesh`))
  (bind _returnvalue (`PrimitiveComponent.CreateDynamicMaterialInstance` _mesh 0 (`PrimitiveComponent.GetMaterial` _mesh 0)))
  (bind _output_get (set `self.DamageMaterial` _returnvalue))
  (bind _returnvalue_2 (`MaterialInstanceDynamic.K2_GetVectorParameterValue` _output_get "BodyColor"))
  (set `self.OriginalColor` (make `LinearColor` (break `LinearColor` _returnvalue_2) (`.G` (break `LinearColor` _returnvalue_2)) (`.B` (break `LinearColor` _returnvalue_2)) (`.A` (break `LinearColor` _returnvalue_2))))
  (set `self.DistToFullRed` (- 1.0 (break `LinearColor` _returnvalue_2)))
  (if (< (`self.CurrentHealth`) 0.0)
    (set `self.CurrentHealth` (`self.MaxHealth`))))

(event `self.ReceivePointDamage`
  (params (Damage :type "Float (single-precision)") (DamageType :type "DamageType Object Reference") (HitLocation :type "Vector Structure") (HitNormal :type "Vector Structure") (HitComponent :type "PrimitiveComponent Object Reference") (BoneName :type Name) (ShotFromDirection :type "Vector Structure") (InstigatedBy :type "Controller Object Reference") (DamageCauser :type "Actor Object Reference") (HitInfo :type "HitResult Structure (by ref)"))
  (`self.Damage` Damage))

(event `Move`
  (params (Direction :type "Vector Structure") (Scale :type "Float (double-precision)"))
  ;[1 1 1] Movement
  (`self.BranchOnDodging`
    (:`false`
      (`self.AddMovementInput` Direction Scale))))

(event `Dodge`
  (`self.CanDodge?`
    (:`True`
      (`self.DodgeLaunch`)
      (`KismetSystemLibrary.K2_SetTimerDelegate` (delegate `DodgeEnd`) (`self.DodgeDuration`))
      (`/Engine/EditorBlueprintResources/StandardMacros.IncrementInt` (`self.DodgeCount`)
        (:`  `
          (`self.PrintDodgeCount`)
          (if (not (`KismetSystemLibrary.K2_IsTimerActiveHandle` (`self.DodgeRefreshTimer`)))
            (bind _returnvalue (`KismetSystemLibrary.K2_SetTimerDelegate` (delegate `RefreshDodge`) (`self.TimeToDodgeRefresh`)))
            (set `self.DodgeRefreshTimer` _returnvalue)))))))

(event `DodgeEnd`
  (`self.SetDodging` false))

(event `RefreshDodge`
  (bind _result (`/Engine/EditorBlueprintResources/StandardMacros.DecrementInt` (`self.DodgeCount`))
    (:`  `
      (`self.PrintDodgeCount`)
      (if (> _result 0)
        (`KismetSystemLibrary.K2_SetTimerDelegate` (delegate `RefreshDodge`) (`self.TimeToDodgeRefresh`))))))

(event `PrimaryShortPress`
  (`self.PrimaryAttack`))

(event `PrimaryLongPress`
  (bind _returnvalue (`self.K2_GetActorLocation`))
  (bind _returnvalue_2 (`GameplayStatics.GetWorldDeltaSeconds`))
  (bind _returnvalue_3 (/ (`self.CloseGapBaseInterpSpeed`) (`self.CloseGapTime`)))
  (bind (_out_hit_distance _target) (`self.CheckForMeleeTarget`))
  (`/Engine/EditorBlueprintResources/StandardMacros.IsValid` _target
    (:`Is Valid`
      (`TimelineComponent.SetTimelineLength` (`self.CloseGap`) (`self.CloseGapTime`))
      (`Timeline|CloseGap` :!via `PlayFromStart`
        (:`Update`
          (bind _returnvalue_4 (`self.K2_GetActorLocation` _target))
          (bind (_returnvalue_roll _returnvalue_pitch _returnvalue_yaw) (`KismetMathLibrary.BreakRotator` (`KismetMathLibrary.FindLookAtRotation` _returnvalue _returnvalue_4)))
          (`self.K2_SetActorLocationAndRotation` (`KismetMathLibrary.VInterpTo` _returnvalue (+ (* (`KismetMathLibrary.Normal` (- _returnvalue _returnvalue_4)) (`self.PrimaryAttackRange`)) _returnvalue_4) _returnvalue_2 _returnvalue_3) (`KismetMathLibrary.RInterpTo` (`self.K2_GetActorRotation`) (`KismetMathLibrary.MakeRotator` 0.0 0.0 _returnvalue_yaw) _returnvalue_2 _returnvalue_3))
          (if (>= (`/Game/BluePrints/Utility/TimelineFunctions.GetCompletionRatio` (`self.CloseGap`)) 0.5)
            (`/Engine/EditorBlueprintResources/StandardMacros.DoOnce` false :!label _label
              (:`Completed`
                (`self.PrimaryAttack`)))))
        (:`Finished`
          (goto _label :!via `Reset`))))
    (:`Is Not Valid`
      (if (`NavMovementComponent.IsFalling` (`self.CharacterMovement`))
        (bind (_out_hit_distance_2 _out_hit_hit_actor) (`self.DiveTargetCheck`))
        (`/Engine/EditorBlueprintResources/StandardMacros.IsValid` _out_hit_hit_actor
          (:`Is Valid`
            (`self.DiveAttack`)))
        (else
          (`self.PrimaryAttack`))))))

(event `InputAction|PrimaryAction`
  (params (Key :type "Key Structure"))
  (:`Pressed`
    (if (not (`self.isAttacking?`))
      (`self.HandleLongPress` (delegate `PrimaryLongPress`) (`self.MeleeLongPressTime`) :!label _label_2
        (:`Exit`
          (if (not (`self.isPrimed?`))
            (set `self.isPrimed?` true)
            (`/Game/Animation/AnimationBPs/RunescaperAnimBP.PrimaryActionPressed` (`self.GetAnimationBP`) (`self.PrimaryAttackMontage`))))
        (:`ShortPress`
          (`self.PrimaryShortPress`)))))
  (:`Released`
    (goto _label_2 :!via `Released`)))

(event `PrimaryAttack`
  (set `self.isPrimed?` false)
  (set `self.isAttacking?` true)
  (`/Game/Animation/AnimationBPs/RunescaperAnimBP.PrimaryActionReleased` (`self.GetAnimationBP`))
  (`self.DrawPrimaryAttackRange`))

(event `OnAttackEnd`
  (set `self.isAttacking?` false))

(event `self.fist_r.OnComponentBeginOverlap`
  (params (OverlappedComponent :type "PrimitiveComponent Object Reference") (OtherActor :type "Actor Object Reference") (OtherComp :type "PrimitiveComponent Object Reference") (OtherBodyIndex :type Integer) (bFromSweep :type Boolean) (SweepResult :type "HitResult Structure (by ref)"))
  (`self.ApplyHitDamage` OtherActor SweepResult)
  (bind _returnvalue (`PrimitiveComponent.GetPhysicsLinearVelocity` (`self.fist_r`) "None"))
  (`KismetSystemLibrary.PrintString` (`KismetStringLibrary.Conv_DoubleToString` (`KismetMathLibrary.VSize` _returnvalue))))

(fn `Aim`
  (params (ForwardAxis :type "Float (double-precision)") (RightAxis :type "Float (double-precision)"))
  (bind _returnvalue (`self.CheckJoystickActive` ForwardAxis RightAxis))
  (`|ExecutionSequence`
    (:`then_0`
      (if _returnvalue
        (`Controller.SetControlRotation` (`self.GetController`) (`self.AxisToCameraSpaceRotation` ForwardAxis RightAxis))))
    (:`then_1`
      (set `CharacterMovementComponent.bOrientRotationToMovement` (not _returnvalue) (`self.CharacterMovement`)))
    (:`then_2`
      (set `self.isAiming?` _returnvalue))))

(fn `ApplyHitDamage`
  (params (DamagedActor :type "Actor Object Reference") (HitInfo :type "HitResult Structure (by ref)"))
  (if (and (!= DamagedActor self) (`self.isAttacking?`))
    (bind _returnvalue (`GameplayStatics.ApplyPointDamage` DamagedActor 10.0 (`KismetMathLibrary.GetDirectionUnitVector` (`self.K2_GetActorLocation` DamagedActor) (`self.K2_GetActorLocation` self)) HitInfo null self))
    (`self.DebugHitDamage` DamagedActor _returnvalue)
    (return)))

(fn `Attack`
  (params (Vulnerability :type "/Game/Data/Enums/EVulnerabilities Enum" :default "NewEnumerator2") (Target :type "Actor Object Reference")))

(fn `AxisHasInput?`
  (params (AxisInput :type "Float (double-precision)"))
  (returns (ReturnValue :type Boolean))
  (return (>= (`KismetMathLibrary.Abs` AxisInput) (`self.RotationDeadzone`))))

(fn `AxisToCameraSpaceRotation`
  (params (ForwardAxis :type "Float (double-precision)") (RightAxis :type "Float (double-precision)"))
  (returns (Rotation :type "Rotator Structure"))
  (bind (_forward _right) (`self.GetProjectedCameraVectors`))
  (return (`KismetMathLibrary.Conv_VectorToRotator` (+ (* _forward ForwardAxis) (* _right RightAxis)))))

(fn `CheckForMeleeTarget`
  (returns (`Out Hit Distance` :type "Float (double-precision)") (Target :type "Actor Object Reference"))
  (bind _capsulecomponent (`self.CapsuleComponent`))
  (bind _returnvalue (`SceneComponent.GetForwardVector` (`self.CapsuleComponent`)))
  (`|ExecutionSequence`
    (:`then_0`
      (bind (_outhit_distance _outhit_hitactor) (`self.MeleeRangeCheck` _returnvalue))
      (`/Engine/EditorBlueprintResources/StandardMacros.IsValid` _outhit_hitactor
        (:`Is Valid`
          (if (`Actor.bCanBeDamaged` _outhit_hitactor)
            (return _outhit_distance _outhit_hitactor)))))
    (:`then_1`
      (bind (_outhit_distance_2 _outhit_hitactor_2) (`self.MeleeRangeCheck` (`KismetMathLibrary.RotateAngleAxis` _returnvalue (`self.MeleeRangeCheckElevationAngle`) (`SceneComponent.GetRightVector` _capsulecomponent))))
      (`/Engine/EditorBlueprintResources/StandardMacros.IsValid` _outhit_hitactor_2
        (:`Is Valid`
          (if (`Actor.bCanBeDamaged` _outhit_hitactor_2)
            (return _outhit_distance_2 _outhit_hitactor_2)))))
    (:`then_2`
      (if (not (`NavMovementComponent.IsFalling` (`self.CharacterMovement`)))
        (bind (_outhit_distance_3 _outhit_hitactor_3) (`self.MeleeRangeCheck` (`KismetMathLibrary.RotateAngleAxis` _returnvalue (* (`self.MeleeRangeCheckElevationAngle`) -1.0) (`SceneComponent.GetRightVector` _capsulecomponent))))
        (`/Engine/EditorBlueprintResources/StandardMacros.IsValid` _outhit_hitactor_3
          (:`Is Valid`
            (if (`Actor.bCanBeDamaged` _outhit_hitactor_3)
              (return _outhit_distance_3 _outhit_hitactor_3))))))
    (:`then_3`
      (return 0.0 null))))

(fn `CheckJoystickActive`
  (params (Vertical :type "Float (double-precision)") (Horizontal :type "Float (double-precision)"))
  (returns (ReturnValue :type Boolean))
  (return (or (`self.AxisHasInput?` Vertical) (`self.AxisHasInput?` Horizontal))))

(fn `Damage`
  (params (value :type "Float (double-precision)"))
  (set `self.CurrentHealth` (- (`self.CurrentHealth`) value))
  (`self.UpdateDamageColor`)
  (if (<= (`self.CurrentHealth`) 0.0)
    (`self.Die`)))

(fn `DebugHitDamage`
  (params (Object :type "Object Object Reference") (InFloat :type "Float (double-precision)"))
  (`KismetSystemLibrary.PrintString` (`KismetStringLibrary.BuildString_Double` "Hit " (`KismetStringLibrary.Concat_StrStr` (`KismetSystemLibrary.GetDisplayName` Object) " for ") InFloat " damage")))

(fn `Die`
  (bind _capsulecomponent (`self.CapsuleComponent`))
  (`self.DisableInput` (`self.GetController`) null)
  (`CharacterMovementComponent.DisableMovement` (`self.CharacterMovement`))
  (bind _returnvalue (`SceneComponent.K2_AttachToComponent` (`self.Mesh`) (`self.RootComponent`) "None" "KeepWorld" "KeepWorld" "KeepWorld" false))
  (`KismetSystemLibrary.PrintString` "Hello" _returnvalue)
  (`ActorComponent.Deactivate` _capsulecomponent)
  (`PrimitiveComponent.SetCollisionEnabled` _capsulecomponent "NoCollision")
  (`self.EnableRagDoll`)
  (`PrimitiveComponent.SetCollisionResponseToChannel` (`self.Mesh`) "ECC_GameTraceChannel1" "ECR_Ignore"))

(fn `DiveAttack`)

(fn `DiveTargetCheck`
  (returns (`Out Hit Distance` :type "Float (double-precision)") (`Out Hit Hit Actor` :type "Actor Object Reference"))
  (bind _capsulecomponent (`self.CapsuleComponent`))
  (bind _returnvalue (`SceneComponent.K2_GetComponentLocation` _capsulecomponent))
  (bind _returnvalue_2 (`KismetMathLibrary.NegateVector` (`SceneComponent.GetUpVector` _capsulecomponent)))
  (bind _outhit (`KismetSystemLibrary.SphereTraceSingle` :`Start` (+ (* _returnvalue_2 (+ (`CapsuleComponent.GetScaledCapsuleRadius` _capsulecomponent) (`self.TargetCheckRadius`))) _returnvalue) :`End` (+ (* _returnvalue_2 (`self.DiveCheckRange`)) _returnvalue) :`Radius` (`self.TargetCheckRadius`) :`TraceChannel` "TraceTypeQuery3" :`DrawDebugType` "ForDuration"))
  (return (`.Distance` (`GameplayStatics.BreakHitResult` _outhit)) (`.HitActor` (`GameplayStatics.BreakHitResult` _outhit))))

(fn `DodgeLaunch`
  (bind _output_get (set `self.DodgeDirection` (`self.GetAxisInputDirection` (`self.GetInputAxisValue`) (`self.GetInputAxisValue`))))
  (`self.SetDodging` true)
  (`self.LaunchCharacter` (* _output_get (`self.GetDodgeSpeed`)) true))

(fn `EnableRagDoll`
  (bind _mesh (`self.Mesh`))
  (`PrimitiveComponent.SetSimulatePhysics` _mesh true)
  (`PrimitiveComponent.SetCollisionEnabled` _mesh "QueryAndPhysics")
  (`PrimitiveComponent.SetCollisionResponseToChannel` _mesh "ECC_Pawn" "ECR_Block"))

(fn `GetAnimationBP`
  (returns (AnimBP :type "/Game/Animation/AnimationBPs/RunescaperAnimBP Object Reference"))
  (bind _asrunescaper_anim_bp (cast `/Game/Animation/AnimationBPs/RunescaperAnimBP` (`SkeletalMeshComponent.GetAnimInstance` (`self.Mesh`))))
  (return _asrunescaper_anim_bp))

(fn `GetAxisInputDirection`
  (params (Vertical :type "Float (double-precision)") (Horizontal :type "Float (double-precision)"))
  (returns (Direction :type "Vector Structure"))
  (if (`self.CheckJoystickActive` Vertical Horizontal)
    (return (`KismetMathLibrary.Normal` (`KismetMathLibrary.MakeVector` Vertical Horizontal)))
    (else
      (return (`KismetMathLibrary.Normal` (`self.GetActorForwardVector`))))))

(fn `GetDodgeSpeed`
  (returns (Speed :type "Float (double-precision)"))
  (return (* (`MovementComponent.GetMaxSpeed` (`self.CharacterMovement`)) (`self.DodgeSpeedMultiplier`))))

(fn `GetProjectedCameraVectors`
  (returns (Forward :type "Vector Structure") (Right :type "Vector Structure"))
  (bind _returnvalue (`KismetMathLibrary.MakeRotator` 0.0 0.0 (.yaw (`PlayerCameraManager.GetCameraRotation` (`GameplayStatics.GetPlayerCameraManager` 0)))))
  (return (`KismetMathLibrary.GetForwardVector` _returnvalue) (`KismetMathLibrary.GetRightVector` _returnvalue)))

(fn `GetRightAxisMagnitude`
  (returns (magnitude :type "Float (double-precision)"))
  (return (`KismetMathLibrary.VSize2D` (`KismetMathLibrary.MakeVector2D` (`self.GetInputAxisValue`) (`self.GetInputAxisValue`)))))

(fn `MeleeRangeCheck`
  (params (Direction :type "Vector Structure"))
  (returns (OutHit_Distance :type "Float (double-precision)") (OutHit_HitActor :type "Actor Object Reference"))
  (bind _capsulecomponent (`self.CapsuleComponent`))
  (bind _returnvalue (`SceneComponent.K2_GetComponentLocation` _capsulecomponent))
  (bind _outhit (`KismetSystemLibrary.SphereTraceSingle` :`Start` (+ (* Direction (+ (`CapsuleComponent.GetScaledCapsuleRadius` _capsulecomponent) (`self.TargetCheckRadius`))) _returnvalue) :`End` (+ (* Direction (`self.TargetCheckRange`)) _returnvalue) :`Radius` (`self.TargetCheckRadius`) :`TraceChannel` "TraceTypeQuery3" :`DrawDebugType` "ForDuration"))
  (return (`.Distance` (`GameplayStatics.BreakHitResult` _outhit)) (`.HitActor` (`GameplayStatics.BreakHitResult` _outhit))))

(fn `SetDodging`
  (params (Condition :type Boolean))
  (bind _output_get (set `self.isDodging?` Condition))
  (if _output_get
    (`self.SetGroundSlowdown` (`self.DodgeGroundFriction`) (`self.DodgeGroundDeceleration`) (`self.DodgeAirDeceleration`))
    (else
      (`self.SetGroundSlowdown` (`self.BaseGroundFriction`) (`self.BaseGroundDeceleration`) (`self.BaseAirDeceleration`))))
  (return))

(fn `UpdateDamageColor`
  (bind _damagematerial (`self.DamageMaterial`))
  (bind _returnvalue (/ (`self.CurrentHealth`) (`self.MaxHealth`)))
  (bind (_r _g _b) (break `LinearColor` (* (`self.OriginalColor`) _returnvalue)))
  (`MaterialInstanceDynamic.K2_GetVectorParameterValue` _damagematerial "BodyColor")
  (`MaterialInstanceDynamic.SetVectorParameterValue` _damagematerial "BodyColor" (make `LinearColor` (- 1.0 (* (`self.DistToFullRed`) _returnvalue)) _g _b)))

(fn `UserConstructionScript`
  (bind _charactermovement (`self.CharacterMovement`))
  (set `CharacterMovementComponent.BrakingDecelerationWalking` (`self.BaseGroundDeceleration`) _charactermovement)
  (set `CharacterMovementComponent.GroundFriction` (`self.BaseGroundFriction`) _charactermovement))