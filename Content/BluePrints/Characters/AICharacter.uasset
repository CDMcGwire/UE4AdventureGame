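; AI character Blueprint that tracks health, tints redder as it takes damage and destroys itself at zero health.
; BeginPlay creates a dynamic material from the mesh's first slot, caches its BodyColor, and sets CurrentHealth to MaxHealth only if it is negative.
; Point damage lowers health, then rescales BodyColor by the remaining fraction, raising red toward full while green and blue fade.
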(event `self.ReceiveBeginPlay`
  (bind _mesh (`self.Mesh`))
  (bind _returnvalue (`PrimitiveComponent.CreateDynamicMaterialInstance` _mesh 0 (`PrimitiveComponent.GetMaterial` _mesh 0)))
  (bind _output_get (set `self.DamageMaterial` _returnvalue))
  (bind _returnvalue_2 (`MaterialInstanceDynamic.K2_GetVectorParameterValue` _output_get "BodyColor"))
  (set `self.OriginalColor` (make `LinearColor` (break `LinearColor` _returnvalue_2) (`.G` (break `LinearColor` _returnvalue_2)) (`.B` (break `LinearColor` _returnvalue_2)) (`.A` (break `LinearColor` _returnvalue_2))))
  (set `self.DistToFullRed` (- 1.0 (break `LinearColor` _returnvalue_2)))
  (if (< (`self.CurrentHealth`) 0.0)
    (set `self.CurrentHealth` (`self.MaxHealth`))))

(event `self.ReceivePointDamage`
  (params (Damage :type "Float (single-precision)") (DamageType :type "DamageType Object Reference") (HitLocation :type "Vector Structure") (HitNormal :type "Vector Structure") (HitComponent :type "PrimitiveComponent Object Reference") (BoneName :type Name) (ShotFromDirection :type "Vector Structure") (InstigatedBy :type "Controller Object Reference") (DamageCauser :type "Actor Object Reference") (HitInfo :type "HitResult Structure (by ref)"))
  (set `self.CurrentHealth` (- (`self.CurrentHealth`) Damage))
  (`self.UpdateDamageColor`)
  (if (<= (`self.CurrentHealth`) 0.0)
    (`self.K2_DestroyActor`)))

(fn `UpdateDamageColor`
  (bind _damagematerial (`self.DamageMaterial`))
  (bind _returnvalue (/ (`self.CurrentHealth`) (`self.MaxHealth`)))
  (bind (_r _g _b) (break `LinearColor` (* (`self.OriginalColor`) _returnvalue)))
  (`MaterialInstanceDynamic.K2_GetVectorParameterValue` _damagematerial "BodyColor")
  (`MaterialInstanceDynamic.SetVectorParameterValue` _damagematerial "BodyColor" (make `LinearColor` (- 1.0 (* (`self.DistToFullRed`) _returnvalue)) _g _b)))

(fn `UserConstructionScript`)