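; Shared player camera that keeps all ThirdPersonCharacters in view by following their average location.
; Each tick it sets the spring arm length from the furthest player's distance plus a margin, never below a minimum.
; A zoom ratio derived once at BeginPlay from pitch, FOV and camera height converts that distance to arm length.
; Rotation events yaw the arm or tilt it within pitch limits.
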(event `self.ReceiveBeginPlay`
  (bind _outactors (`GameplayStatics.GetAllActorsOfClass` "/Game/BluePrints/Characters/ThirdPersonCharacter.ThirdPersonCharacter_C"))
  (set `self.Players` _outactors)
  (`self.CalculateCameraBlindspot`))

(event `self.ReceiveTick`
  (params (DeltaSeconds :type "Float (single-precision)"))
  (bind _returnvalue (`GameplayStatics.GetActorArrayAverageLocation` (`self.Players`)))
  (`self.K2_SetActorLocation` _returnvalue)
  (bind _distance (`self.GetFurthestPlayer`))
  (`self.AdjustHeight` _distance))

(event `RotateHorizontal`
  (params (Delta :type "Float (double-precision)"))
  (`SceneComponent.K2_AddWorldRotation` (`self.SpringArm`) (`KismetMathLibrary.MakeRotator` 0.0 0.0 Delta) false false))

(event `RotateVertical`
  (params (Delta :type "Float (double-precision)"))
  (`self.TiltCameraWithClamp` Delta))

(fn `AdjustHeight`
  (params (FurthestPlayer :type "Float (double-precision)"))
  (bind _minarmlength (`self.MinArmLength`))
  (bind _returnvalue (* (+ FurthestPlayer (`self.ZoomMargin`)) (`self.BlindspotToArmLengthRatio`)))
  (if (> _returnvalue _minarmlength)
    (set `SpringArmComponent.TargetArmLength` _returnvalue (`self.SpringArm`))
    (else
      (set `SpringArmComponent.TargetArmLength` _minarmlength (`self.SpringArm`)))))

(fn `CalculateCameraBlindspot`
  (bind _camera (`self.Camera`))
  (bind (_returnvalue_x _returnvalue_y _returnvalue_z) (`KismetMathLibrary.BreakVector` (`SceneComponent.K2_GetComponentLocation` _camera)))
  (bind (_returnvalue_x_2 _returnvalue_y_2 _returnvalue_z_2) (`KismetMathLibrary.BreakVector` (`SceneComponent.K2_GetComponentLocation` (`self.DefaultSceneRoot`))))
  (bind _output_get (set `self.DistanceToBlindspot` (- (`KismetMathLibrary.VSize2D` (- (`KismetMathLibrary.MakeVector2D` _returnvalue_x _returnvalue_y) (`KismetMathLibrary.MakeVector2D` _returnvalue_x_2 _returnvalue_y_2))) (* (`KismetMathLibrary.DegTan` (- (- 90.0 (`KismetMathLibrary.Abs` (.pitch (`SceneComponent.RelativeRotation` (`self.SpringArm`))))) (/ (/ (`CameraComponent.FieldOfView` _camera) (`CameraComponent.AspectRatio` _camera)) 2.0))) (- _returnvalue_z _returnvalue_z_2)))))
  (set `self.BlindspotToArmLengthRatio` (/ (`self.MinArmLength`) _output_get))
  (return))

(fn `GetCameraWorldRotation`
  (returns (ReturnValue :type "Rotator Structure"))
  (return (`SceneComponent.K2_GetComponentRotation` (`self.Camera`))))

(fn `GetFurthestPlayer`
  (returns (Distance :type "Float (double-precision)"))
  (locals (Furthest :type "Float (double-precision)"))
  (for _array_element (`self.Players`)
    (`/Engine/EditorBlueprintResources/StandardMacros.IsValid` _array_element
      (:`Is Valid`
        (bind _returnvalue (`self.GetDistanceTo` _array_element self))
        (if (> _returnvalue (`local.Furthest`))
          (set `local.Furthest` _returnvalue)))))
  (return (`local.Furthest`)))

(fn `TiltCameraWithClamp`
  (params (Delta :type "Float (double-precision)"))
  (bind _springarm (`self.SpringArm`))
  (bind (_relativerotation_roll _relativerotation_pitch _relativerotation_yaw) (`KismetMathLibrary.BreakRotator` (`SceneComponent.RelativeRotation` _springarm)))
  (`SceneComponent.K2_SetRelativeRotation` _springarm (`KismetMathLibrary.MakeRotator` _relativerotation_roll (`KismetMathLibrary.ClampAngle` (+ (* Delta -1.0) _relativerotation_pitch) (* (`self.MaxCameraPitch`) -1.0) (* (`self.MinCameraPitch`) -1.0)) _relativerotation_yaw) false false))

(fn `UserConstructionScript`)