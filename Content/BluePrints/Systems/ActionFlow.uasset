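; ActionFlow sequences an owner's actions from press and release events, holding one current action and one buffered next action.
; A press primes the action if none is current and CanAct passes; otherwise a different action is buffered.
; Tick updates the current action until its release clears it, then primes the buffered one, keeping it current only if still held.
; Buffer decay compares the fixed NextDecayTime, so its timer never accumulates.
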(event `Event Press`
  (params (Action :type "/Game/BluePrints/Systems/Action Object Reference"))
  (bind _currentaction (`self.CurrentAction`))
  (`/Engine/EditorBlueprintResources/StandardMacros.IsValid` _currentaction
    (:`Is Valid`
      (if (== _currentaction Action)
        (`KismetSystemLibrary.PrintString` "WARNING - Tried to start an action that action that was already current." false true (struct :`R` 1.0 :`G` 0.355096 :`A` 1.0))
        (else
          (set `self.NextAction` Action)
          (set `self.NextDecayTimer` (`self.NextDecayTime`))
          (set `self.NextReleased` false))))
    (:`Is Not Valid`
      (if (`/Game/BluePrints/Systems/Action.CanAct?` Action (`self.GetOwner`))
        (bind _output_get (set `self.CurrentAction` Action))
        (`/Game/BluePrints/Systems/Action.Prime` _output_get)))))

(event `self.ReceiveTick`
  (params (DeltaSeconds :type "Float (single-precision)"))
  (bind _currentaction (`self.CurrentAction`))
  (bind _nextdecaytime (`self.NextDecayTime`))
  (bind _nextaction (`self.NextAction`))
  (`/Engine/EditorBlueprintResources/StandardMacros.IsValid` _currentaction
    (:`Is Valid`
      (`/Game/BluePrints/Systems/Action.Update` _currentaction DeltaSeconds)
      (`/Engine/EditorBlueprintResources/StandardMacros.IsValid` (`self.NextAction`)
        (:`Is Valid`
          (set `self.NextDecayTimer` (- _nextdecaytime DeltaSeconds))
          (if (<= _nextdecaytime 0.0)
            (set `self.NextAction` null)
            (set `self.NextReleased` false :!label _label)))))
    (:`Is Not Valid`
      (`/Engine/EditorBlueprintResources/StandardMacros.IsValid` _nextaction
        (:`Is Valid`
          (`/Game/BluePrints/Systems/Action.Prime` _nextaction)
          (if (not (`self.NextReleased`))
            (set `self.CurrentAction` (`self.NextAction`)))
          (set `self.NextAction` null)
          (goto _label))))))

(event `Event Release`
  (params (Action :type "/Game/BluePrints/Systems/Action Object Reference"))
  (bind _nextaction (`self.NextAction`))
  (bind _currentaction (`self.CurrentAction`))
  (`/Engine/EditorBlueprintResources/StandardMacros.IsValid` _currentaction
    (:`Is Valid`
      (if (== _currentaction Action)
        (`/Game/BluePrints/Systems/Action.Release` (`self.CurrentAction`))
        (set `self.CurrentAction` null)
        (else
          (`/Engine/EditorBlueprintResources/StandardMacros.IsValid` _nextaction :!label _label_2
            (:`Is Valid`
              (if (== _nextaction Action)
                (set `self.NextReleased` true)))))))
    (:`Is Not Valid`
      (goto _label_2))))